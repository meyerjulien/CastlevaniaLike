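; BP_EnemyPatrolBox is an overlap area that tells a group of patrolling enemies when the player enters or leaves it.
; Begin and end overlap events identify the player by checking the other actor for BPI_Player.
; On entry, every actor in PatrolActors receives the player as combat target through SetCombatTargetMessage.
; On exit, the same message is sent with no target, clearing it.
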(event `self.ReceiveActorBeginOverlap`
  (params (OtherActor :type "Actor Object Reference"))
  ;[1 1 1] Is Overlapping Actor the Player?
  (if (`KismetSystemLibrary.DoesImplementInterface` OtherActor "/Game/Blueprints/Interfaces/BPI_Player.BPI_Player_C")
    ;[1 1 1] Set Combat Target as Player for each Patroling Actors
    (for _array_element (`self.PatrolActors`)
      (message `/Game/Blueprints/Interfaces/BPI_Enemy.SetCombatTarget` _array_element OtherActor))))

(event `self.ReceiveActorEndOverlap`
  (params (OtherActor :type "Actor Object Reference"))
  ;[1 1 1] Is End Overlapping Actor the Player?
  (if (`KismetSystemLibrary.DoesImplementInterface` OtherActor "/Game/Blueprints/Interfaces/BPI_Player.BPI_Player_C")
    ;[1 1 1] Set Combat Target as NOTHING for each Patroling Actors
    (for _array_element (`self.PatrolActors`)
      (message `/Game/Blueprints/Interfaces/BPI_Enemy.SetCombatTarget` _array_element null))))

(fn `UserConstructionScript`)