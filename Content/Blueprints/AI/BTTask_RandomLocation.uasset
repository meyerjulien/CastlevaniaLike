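; Behavior Tree task that picks a random wander location for an AI pawn, constrained to the pawn's current Y plane.
; It takes X and Z from random reachable navmesh points around the pawn and keeps the pawn's own Y.
; The result is briefly shown as a debug sphere, written to a Blackboard vector key, and the task finishes successfully.
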(event `self.ReceiveExecuteAI`
  (params (OwnerController :type "AIController Object Reference") (ControlledPawn :type "Pawn Object Reference"))
  (bind _returnvalue (`Actor.K2_GetActorLocation` ControlledPawn))
  (bind _output_get (set `self.RandomLocation` (`KismetMathLibrary.MakeVector` (.x (`NavigationSystemV1.K2_GetRandomReachablePointInRadius` _returnvalue 2500.0 null null)) (.y _returnvalue) (.z (`NavigationSystemV1.K2_GetRandomReachablePointInRadius` _returnvalue 2500.0 null null)))))
  (`KismetSystemLibrary.DrawDebugSphere` _output_get 20.0 12 (struct :`R` 1.0 :`G` 0.033202 :`A` 1.0) 2.0)
  (`BTFunctionLibrary.SetBlackboardValueAsVector` (`self.BBKey_Location`) (`self.RandomLocation`))
  (`self.FinishExecute` true))