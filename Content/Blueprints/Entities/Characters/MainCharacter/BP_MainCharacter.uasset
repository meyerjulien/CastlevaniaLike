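; Player character for a 2D side-scroller using PaperZD, with Enhanced Input movement, jumping and a three-hit melee combo.
; Movement runs along the X axis, flipping controller yaw by acceleration direction, and is blocked with jumping while attacking.
; Attack input during an open window queues the next hit, which ResetAttacking plays as an animation override.
; It creates the overlay widget on BeginPlay and updates its health bar when damaged.
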(event `self.ReceiveTick`
  (params (DeltaSeconds :type "Float (single-precision)")))

(event `self.ReceiveBeginPlay`
  (`parent.ReceiveBeginPlay`)
  (`self.AddMappingContext`)
  (`self.CreateOverlay`))

(event `EnhancedInput|/Game/Inputs/InputActions/IA_Move`
  (params (ActionValue :type "Float (double-precision)") (ElapsedSeconds :type "Float (double-precision)") (TriggeredSeconds :type "Float (double-precision)") (InputAction :type "InputAction Object Reference" :default "/Game/Inputs/InputActions/IA_Move.IA_Move"))
  (:`Triggered`
    (if (not (`self.IsAttacking`))
      (`self.RotateController`)
      (`self.AddMovementInput` (1.0 0.0 0.0) (`KismetMathLibrary.Conv_IntToDouble` (`KismetMathLibrary.Round` ActionValue))))))

(event `EnhancedInput|/Game/Inputs/InputActions/IA_Jump`
  (params (ActionValue :type Boolean) (ElapsedSeconds :type "Float (double-precision)") (TriggeredSeconds :type "Float (double-precision)") (InputAction :type "InputAction Object Reference" :default "/Game/Inputs/InputActions/IA_Jump.IA_Jump"))
  (:`Started`
    (if (not (`self.IsAttacking`))
      (`self.Jump`))))

(event `EnhancedInput|/Game/Inputs/InputActions/IA_Attack`
  (params (ActionValue :type Boolean) (ElapsedSeconds :type "Float (double-precision)") (TriggeredSeconds :type "Float (double-precision)") (InputAction :type "InputAction Object Reference" :default "/Game/Inputs/InputActions/IA_Attack.IA_Attack"))
  (:`Triggered`
    (if (`self.AttackWindowOpen`)
      (set `self.ComboActivated` true)
      (elif (not (`self.IsAttacking`))
        (set `self.IsAttacking` true)
        (`PaperZDAnimInstance.K2_PlayAnimationOverride` (`PaperZDAnimationComponent.AnimInstance` (`self.PaperZDAnimation`)) "/Game/Blueprints/Entities/Characters/MainCharacter/AnimSequences/Attack1.Attack1" "DefaultSlot" 1.0 0.0)))))

(event `/Game/Blueprints/Interfaces/BPI_Player.SetAttackWindow`
  (params (Open :type Boolean))
  (bind _output_get (set `self.AttackWindowOpen` Open))
  (`KismetSystemLibrary.PrintString` (`KismetStringLibrary.Conv_BoolToString` _output_get)))

(event `/Game/Blueprints/Interfaces/BPI_Player.ResetAttacking`
  (if (`self.ComboActivated`)
    ;[1 1 1] Checks Attack count. 'Greather than' value sets the maxium number of attacks that can be done in a combo (2 = total of 3 attacks, 3 = total of 4, etc. It starts at index 0)
    (bind _result (`/Engine/EditorBlueprintResources/StandardMacros.IncrementInt` (`self.AttackCount`))
      (:`  `
        (if (> _result 2)
          (set `self.IsAttacking` false)
          (set `self.AttackCount` 0)
          (set `self.ComboActivated` false)
          (else
            (switch `int` (`self.AttackCount`)
              (:`0`
                (`PaperZDAnimInstance.K2_PlayAnimationOverride` (`PaperZDAnimationComponent.AnimInstance` (`self.PaperZDAnimation`)) "/Game/Blueprints/Entities/Characters/MainCharacter/AnimSequences/Attack1.Attack1" "DefaultSlot" 1.0 0.0)
                (set `self.ComboActivated` false))
              (:`1`
                (`PaperZDAnimInstance.K2_PlayAnimationOverride` (`PaperZDAnimationComponent.AnimInstance` (`self.PaperZDAnimation`)) "/Game/Blueprints/Entities/Characters/MainCharacter/AnimSequences/Attack2.Attack2" "DefaultSlot" 1.0 0.0)
                (set `self.ComboActivated` false))
              (:`2`
                (`PaperZDAnimInstance.K2_PlayAnimationOverride` (`PaperZDAnimationComponent.AnimInstance` (`self.PaperZDAnimation`)) "/Game/Blueprints/Entities/Characters/MainCharacter/AnimSequences/Attack3.Attack3" "DefaultSlot" 1.0 0.0)
                (set `self.ComboActivated` false)))))))
    (else
      (set `self.IsAttacking` false)
      (set `self.AttackCount` 0))))

(fn `AddMappingContext`
  (bind _asplayer_controller (cast `PlayerController` (`self.GetController`)))
  (`EnhancedInputSubsystemInterface.AddMappingContext` (pcsubsystem `EnhancedInputLocalPlayerSubsystem` _asplayer_controller) "/Game/Inputs/IMC_MainCharacter.IMC_MainCharacter" 0 (struct)))

(fn `CreateOverlay`
  (bind _returnvalue (`|CreateWidget` "/Game/Blueprints/UI/WBP_Overlay.WBP_Overlay_C" (cast `PlayerController` (`self.GetController`) :!pure true)))
  (bind _output_get (set `self.Overlay` _returnvalue))
  (`UserWidget.AddToViewport` _output_get 0))

(fn `DecrementHealth`
  (params (Damage :type "Float (double-precision)"))
  (`parent.DecrementHealth` Damage)
  (`/Game/Blueprints/UI/WBP_PlayerHealthBar.UpdateHealth` (`/Game/Blueprints/UI/WBP_Overlay.WBP_PlayerHealthBar` (`self.Overlay`)) (`self.Health`) (`self.MaxHealth`)))

(fn `RotateController`
  (bind _returnvalue_x (`KismetMathLibrary.BreakVector` (`CharacterMovementComponent.GetCurrentAcceleration` (`self.CharacterMovement`))))
  ;[1 1 1] Compare with 0 to determine which direction to look at
  (`/Engine/EditorBlueprintResources/StandardMacros.CompareFloat` _returnvalue_x
    (:`>`
      ;[1 1 1] Default(Do nothing)
      (`Controller.SetControlRotation` (`self.GetController`) (`KismetMathLibrary.MakeRotator` 0.0)))
    (:`<`
      ;[1 1 1] Flips to the other side
      (`Controller.SetControlRotation` (`self.GetController`) (`KismetMathLibrary.MakeRotator` 0.0 0.0 180.0)))))

(fn `UserConstructionScript`)