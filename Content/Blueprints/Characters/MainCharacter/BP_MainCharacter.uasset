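; Player character with side-scrolling style controls: movement along the world X axis and jumping.
; On BeginPlay it adds the IMC_MainCharacter mapping context to the Enhanced Input subsystem.
; IA_Move feeds its rounded value into movement input, while IA_Jump triggers a jump.
; Before each movement input, RotateController snaps control yaw to 0 or 180 from the sign of current X acceleration, leaving it unchanged at zero.
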(event `self.ReceiveBeginPlay`
  (`self.AddMappingContext`))

(event `EnhancedInput|/Game/Inputs/InputActions/IA_Move`
  (params (ActionValue :type "Float (double-precision)") (ElapsedSeconds :type "Float (double-precision)") (TriggeredSeconds :type "Float (double-precision)") (InputAction :type "InputAction Object Reference" :default "/Game/Inputs/InputActions/IA_Move.IA_Move"))
  (:`Triggered`
    (`self.RotateController`)
    (`self.AddMovementInput` (1.0 0.0 0.0) (`KismetMathLibrary.Conv_IntToDouble` (`KismetMathLibrary.Round` ActionValue)))))

(event `EnhancedInput|/Game/Inputs/InputActions/IA_Jump`
  (params (ActionValue :type Boolean) (ElapsedSeconds :type "Float (double-precision)") (TriggeredSeconds :type "Float (double-precision)") (InputAction :type "InputAction Object Reference" :default "/Game/Inputs/InputActions/IA_Jump.IA_Jump"))
  (:`Started`
    (`self.Jump`)))

(fn `AddMappingContext`
  (bind _asplayer_controller (cast `PlayerController` (`self.GetController`)))
  (`EnhancedInputSubsystemInterface.AddMappingContext` (pcsubsystem `EnhancedInputLocalPlayerSubsystem` _asplayer_controller) "/Game/Inputs/IMC_MainCharacter.IMC_MainCharacter" 0 (struct)))

(fn `RotateController`
  (bind _returnvalue_x (`KismetMathLibrary.BreakVector` (`CharacterMovementComponent.GetCurrentAcceleration` (`self.CharacterMovement`))))
  ;[1 1 1] Compare with 0 to determine which direction to look at
  (`/Engine/EditorBlueprintResources/StandardMacros.CompareFloat` _returnvalue_x
    (:`>`
      ;[1 1 1] Default(Do nothing)
      (`Controller.SetControlRotation` (`self.GetController`) (`KismetMathLibrary.MakeRotator` 0.0)))
    (:`<`
      ;[1 1 1] Flips to the other side
      (`Controller.SetControlRotation` (`self.GetController`) (`KismetMathLibrary.MakeRotator` 0.0 0.0 180.0)))))

(fn `UserConstructionScript`)